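; Game mode Blueprint that switches the game between main menu, play and pause states.
; On BeginPlay it creates the main menu, pause menu and play HUD widgets hidden, then enters main menu mode.
; ChangeMode calls a per-state function that toggles widget visibility, game pause, input mode and mouse cursor, then stores the mode.
; Pause is entered only when the game is not already paused, and also hides the HUD's inventory.
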(event Custom|ChangeMode
  (params (GameMode :type GameModes%20Enum :default "NewEnumerator0"))
  ;[1 1 1] Change Game Mode
  (switch Utilities|FlowControl|Switch|SwitchonGameModes GameMode
    (:NewEnumerator0
      (CallFunction|MainMnu)
      (Variables|Default|SetGameMode GameMode :!label _label))
    (:NewEnumerator1
      (CallFunction|InPlay)
      (goto _label))
    (:NewEnumerator2
      (if (not (Game|IsGamePaused))
        (CallFunction|PauseMnu)
        (goto _label)))))

(event EventBeginPlay
  (bind _returnvalue (Game|GetPlayerController 0))
  (Utilities|FlowControl|Sequence
    (:then_0
      (bind _returnvalue_2 (UserInterface|CreateWidget "/Game/NUESTRO/UMG/MainMenuBP.MainMenuBP_C" _returnvalue))
      (bind _output_get (Variables|Default|SetMainMenu _returnvalue_2))
      (UserInterface|Viewport|AddtoViewport _output_get 0)
      (Widget|SetVisibility _output_get "Hidden"))
    (:then_1
      (bind _returnvalue_3 (UserInterface|CreateWidget "/Game/NUESTRO/UMG/PauseMenuBP.PauseMenuBP_C" _returnvalue))
      (bind _output_get_2 (Variables|Default|SetPauseMenu _returnvalue_3))
      (UserInterface|Viewport|AddtoViewport _output_get_2 0)
      (Widget|SetVisibility _output_get_2 "Hidden"))
    (:then_2
      (bind _returnvalue_4 (UserInterface|CreateWidget "/Game/NUESTRO/UMG/PlayBP.PlayBP_C" _returnvalue))
      (bind _output_get_3 (Variables|Default|SetPlayUMG _returnvalue_4))
      (UserInterface|Viewport|AddtoViewport _output_get_3 0)
      (Widget|SetVisibility _output_get_3 "Hidden"))
    (:then_3
      (CallFunction|ChangeMode "NewEnumerator0"))))

(event EventTick
  (params (DeltaSeconds :type Float%20%28single-precision%29)))

(fn ConstructionScript)

(fn MainMnu
  (bind _returnvalue (Game|GetPlayerController 0))
  (Utilities|FlowControl|Sequence
    (:then_0
      (Widget|SetVisibility (Variables|Default|GetPauseMenu) "Hidden"))
    (:then_1
      (Game|SetGamePaused true))
    (:then_2
      (Widget|SetVisibility (Variables|Default|GetPlayUMG) "Hidden"))
    (:then_3
      (Widget|SetVisibility (Variables|Default|GetMainMenu) "Visible")
      (Input|SetInputModeUIOnly _returnvalue 0 "DoNotLock")
      (Variables|/Script/Engine.PlayerController|SetbShowMouseCursor _returnvalue true))))

(fn PauseMnu
  (bind _returnvalue (Game|GetPlayerController 0))
  (bind _playumg (Variables|Default|GetPlayUMG))
  (Utilities|FlowControl|Sequence
    (:then_0
      (Widget|SetVisibility (Variables|Default|GetPauseMenu) "Visible"))
    (:then_1
      (Game|SetGamePaused true)
      (Variables|/Script/Engine.PlayerController|SetbShowMouseCursor _returnvalue true)
      (Input|SetInputModeUIOnly _returnvalue 0 "DoNotLock"))
    (:then_2
      (Widget|SetVisibility _playumg "Hidden")
      (Widget|SetVisibility (Variables|/Game/NUESTRO/UMG/PlayBP.PlayBP_C|GetInventoryBP _playumg) "Hidden"))))

(fn InPlay
  (bind _returnvalue (Game|GetPlayerController 0))
  (Utilities|FlowControl|Sequence
    (:then_0
      (Widget|SetVisibility (Variables|Default|GetMainMenu) "Hidden"))
    (:then_1
      (Widget|SetVisibility (Variables|Default|GetPauseMenu) "Hidden"))
    (:then_2
      (Widget|SetVisibility (Variables|Default|GetPlayUMG) "Visible"))
    (:then_3
      (if (Game|IsGamePaused)
        (Game|SetGamePaused false)))
    (:then_4
      (Input|SetInputModeGameOnly _returnvalue)
      (Variables|/Script/Engine.PlayerController|SetbShowMouseCursor _returnvalue false))))