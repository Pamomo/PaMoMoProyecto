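; Pickup item actor for the inventory, configured by a row name in the ListOfWeapons data table.
; The Construction Script looks up the Identificador row, caches its struct, name, description and icon, and applies its skeletal mesh.
; When MainCharBP overlaps the capsule, the item passes the struct to the character's Recoger function and destroys itself.
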(event OnComponentBeginOverlap(Capsule)
  (params (OverlappedComponent :type Primitive%20Component%20Object%20Reference) (OtherActor :type Actor%20Object%20Reference) (OtherComp :type Primitive%20Component%20Object%20Reference) (OtherBodyIndex :type Integer) (bFromSweep :type Boolean) (SweepResult :type Hit%20Result%20Structure%20%28by%20ref%29))
  (bind _asmain_char_bp (Utilities|Casting|CastToMainCharBP OtherActor))
  (Default|Recoger _asmain_char_bp (Variables|Default|GetMiStruct))
  (Actor|DestroyActor))

(event EventBeginPlay)

(event Collision|EventActorBeginOverlap
  (params (OtherActor :type Actor%20Object%20Reference)))

(event EventTick
  (params (DeltaSeconds :type Float%20%28single-precision%29)))

(fn ConstructionScript
  (bind _returnvalue (Utilities|GetDataTableRow "/Game/NUESTRO/INVENTORY/ListOfWeapons.ListOfWeapons" (Variables|Default|GetIdentificador))
    (:then
      (Variables|Default|SetMiStruct _returnvalue)
      (Variables|Default|SetItem_Name (.Item_Name (Utilities|Struct|BreakArma _returnvalue)))
      (Variables|Default|SetDescription (.Description (Utilities|Struct|BreakArma _returnvalue)))
      (Variables|Default|SetIcono (.Icon (Utilities|Struct|BreakArma _returnvalue)))
      (Class|SkinnedMeshComponent|SetSkeletalMesh (Variables|Default|GetSkeletalMesh) (.Item_Mesh (Utilities|Struct|BreakArma _returnvalue)) true))))