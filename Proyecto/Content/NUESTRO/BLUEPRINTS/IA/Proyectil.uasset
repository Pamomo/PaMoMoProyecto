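; AI projectile actor that damages the player on contact.
; On BeginPlay it launches its StaticMesh with a velocity-change impulse along a Direction scaled by an Impulse strength.
; When its Sphere overlaps MainCharBP, it sends fixed damage to MyGameModeBP through RecibirDaño, then destroys itself.
; Overlaps with any other actor are ignored.
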(event OnComponentBeginOverlap(Sphere)
  (params (OverlappedComponent :type Primitive%20Component%20Object%20Reference) (OtherActor :type Actor%20Object%20Reference) (OtherComp :type Primitive%20Component%20Object%20Reference) (OtherBodyIndex :type Integer) (bFromSweep :type Boolean) (SweepResult :type Hit%20Result%20Structure%20%28by%20ref%29))
  (Utilities|Casting|CastToMainCharBP OtherActor)
  (bind _asmy_game_mode_bp (Utilities|Casting|CastToMyGameModeBP (Game|GetGameMode)))
  (Default|RecibirDaño _asmy_game_mode_bp 3e+01)
  (Actor|DestroyActor))

(event EventBeginPlay
  (Physics|AddImpulse (Variables|Default|GetStaticMesh) (* (Variables|Default|GetDirection) (Variables|Default|GetImpulse)) "None" true))

(fn ConstructionScript)