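; Maestro quest-giver actor that walks the player through a linear quest chain, displaying each quest's narrative text.
; BeginPlay copies QuestDT rows into an array, tracking completion there.
; Player overlap with its box switches on quest number, advancing after a delay or when GameInstance flags are met, the latter granting the next enum-sequenced reward to the character.
; Tick periodically randomizes a Talk value through a gate; GuitarPlayTime toggles around the guitar quest.
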(event OnComponentBeginOverlap(Box)
  (params (OverlappedComponent :type Primitive%20Component%20Object%20Reference) (OtherActor :type Actor%20Object%20Reference) (OtherComp :type Primitive%20Component%20Object%20Reference) (OtherBodyIndex :type Integer) (bFromSweep :type Boolean) (SweepResult :type Hit%20Result%20Structure%20%28by%20ref%29))
  (Utilities|Casting|CastToMainCharBP OtherActor)
  (switch Utilities|FlowControl|Switch|SwitchonQuests (Variables|Default|GetQuest)
    (:NewEnumerator0
      (Utilities|FlowControl|Delay 1e+01)
      (CallFunction|CompleteQuest)
      (CallFunction|CheckQuest)
      (CallFunction|ChangeText))
    (:NewEnumerator1
      (Utilities|FlowControl|Delay 1e+01)
      (CallFunction|CompleteQuest)
      (CallFunction|CheckQuest)
      (CallFunction|ChangeText)
      (Variables|Default|SetGuitarPlayTime true))
    (:NewEnumerator2
      (Variables|Default|SetGuitarPlayTime false)
      (if (Variables|/Game/NUESTRO/BLUEPRINTS/MyGameInstanceBP.MyGameInstanceBP_C|GetGuitarra (.AsMy%20Game%20Instance%20BP (Utilities|Casting|CastToMyGameInstanceBP (Game|GetGameInstance))))
        (CallFunction|CompleteQuest)
        (CallFunction|CheckQuest)
        (Default|RecompensaQuest (.AsMain%20Char%20BP (Utilities|Casting|CastToMainCharBP (Game|GetPlayerCharacter 0))) (Variables|Default|GetRecompensa))
        (bind _siguiente (CallFunction|GetNextEnumIndex (Variables|Default|GetRecompensa)))
        (Variables|Default|SetRecompensa _siguiente)
        (CallFunction|ChangeText)))
    (:NewEnumerator3
      (Utilities|FlowControl|Delay 1e+01)
      (CallFunction|CompleteQuest)
      (CallFunction|CheckQuest)
      (CallFunction|ChangeText))
    (:NewEnumerator4
      (if (Variables|/Game/NUESTRO/BLUEPRINTS/MyGameInstanceBP.MyGameInstanceBP_C|GetBaguete (.AsMy%20Game%20Instance%20BP (Utilities|Casting|CastToMyGameInstanceBP (Game|GetGameInstance))))
        (CallFunction|CompleteQuest)
        (CallFunction|CheckQuest)
        (Default|RecompensaQuest (.AsMain%20Char%20BP (Utilities|Casting|CastToMainCharBP (Game|GetPlayerCharacter 0))) (Variables|Default|GetRecompensa))
        (bind _siguiente_2 (CallFunction|GetNextEnumIndex (Variables|Default|GetRecompensa)))
        (Variables|Default|SetRecompensa _siguiente_2)
        (CallFunction|ChangeText)))
    (:NewEnumerator5
      (if (Variables|/Game/NUESTRO/BLUEPRINTS/MyGameInstanceBP.MyGameInstanceBP_C|GetTodosLosPollos (.AsMy%20Game%20Instance%20BP (Utilities|Casting|CastToMyGameInstanceBP (Game|GetGameInstance))))
        (CallFunction|CompleteQuest)
        (CallFunction|CheckQuest)
        (Default|RecompensaQuest (.AsMain%20Char%20BP (Utilities|Casting|CastToMainCharBP (Game|GetPlayerCharacter 0))) (Variables|Default|GetRecompensa))
        (bind _siguiente_3 (CallFunction|GetNextEnumIndex (Variables|Default|GetRecompensa)))
        (Variables|Default|SetRecompensa _siguiente_3)
        (CallFunction|ChangeText)))
    (:NewEnumerator6
      (Utilities|FlowControl|Delay 1e+01)
      (CallFunction|CompleteQuest)
      (CallFunction|CheckQuest)
      (CallFunction|ChangeText))
    (:NewEnumerator7
      (if (Variables|/Game/NUESTRO/BLUEPRINTS/MyGameInstanceBP.MyGameInstanceBP_C|GetPoderDeLasPerlas (.AsMy%20Game%20Instance%20BP (Utilities|Casting|CastToMyGameInstanceBP (Game|GetGameInstance))))
        (CallFunction|CompleteQuest)
        (CallFunction|CheckQuest)
        (Default|RecompensaQuest (.AsMain%20Char%20BP (Utilities|Casting|CastToMainCharBP (Game|GetPlayerCharacter 0))) (Variables|Default|GetRecompensa))
        (bind _siguiente_4 (CallFunction|GetNextEnumIndex (Variables|Default|GetRecompensa)))
        (Variables|Default|SetRecompensa _siguiente_4)
        (CallFunction|ChangeText)))
    (:NewEnumerator8
      (if (Variables|/Game/NUESTRO/BLUEPRINTS/MyGameInstanceBP.MyGameInstanceBP_C|GetFisioCurado (.AsMy%20Game%20Instance%20BP (Utilities|Casting|CastToMyGameInstanceBP (Game|GetGameInstance))))
        (CallFunction|CompleteQuest)
        (CallFunction|CheckQuest)
        (Default|RecompensaQuest (.AsMain%20Char%20BP (Utilities|Casting|CastToMainCharBP (Game|GetPlayerCharacter 0))) (Variables|Default|GetRecompensa))
        (bind _siguiente_5 (CallFunction|GetNextEnumIndex (Variables|Default|GetRecompensa)))
        (Variables|Default|SetRecompensa _siguiente_5)
        (CallFunction|ChangeText)))))

(event Custom|CheckQuest
  (bind _array_element (Utilities|Array|ForEachLoopwithBreak (Variables|Default|GetMisiones) :!label _label)
    (:LoopBody
      (if (Math|Boolean|Equal(Boolean) (.Completada (Utilities|Struct|BreakQuest _array_element)) false)
        (goto _label Break)))
    (:Completed
      (Variables|Default|SetActualQuest _array_element)
      (Variables|Default|SetQuest (.QuestNumber (Utilities|Struct|BreakQuest _array_element))))))

(event Custom|CompleteQuest
  (bind _misiones (Variables|Default|GetMisiones))
  (|SetBy-RefVar (.Completada (Utilities|Struct|BreakQuest (Utilities|Array|Get(acopy) _misiones (Utilities|Array|FindItem _misiones (Variables|Default|GetActualQuest))))) true))

(event Custom|ChangeText
  (bind _misiones (Variables|Default|GetMisiones))
  (Rendering|Components|TextRender|SetText (Variables|Default|GetInstruccion) (.Narrativa (Utilities|Struct|BreakQuest (Utilities|Array|Get(acopy) _misiones (Utilities|Array|FindItem _misiones (Variables|Default|GetActualQuest)))))))

(event EventBeginPlay
  (bind _outrownames (DataTable|GetDataTableRowNames "/Game/NUESTRO/BLUEPRINTS/QuestDT.QuestDT"))
  (for _array_element _outrownames
    (bind _returnvalue (Utilities|GetDataTableRow "/Game/NUESTRO/BLUEPRINTS/QuestDT.QuestDT" _array_element)
      (:then
        (Utilities|Array|Add (Variables|Default|GetMisiones) _returnvalue)))))

(event EventTick
  (params (DeltaSeconds :type Float%20%28single-precision%29))
  (Utilities|FlowControl|Sequence
    (:then_0
      (Utilities|FlowControl|Gate false :!label _label
        (:Exit
          (if (< (Math|Random|RandomFloatinRange (- (Variables|Default|GetTalk) 25.0) (+ (Variables|Default|GetTalk) 25.0)) 0.0)
            (Variables|Default|SetTalk 0.0)
            (elif (> (Math|Random|RandomFloatinRange (- (Variables|Default|GetTalk) 25.0) (+ (Variables|Default|GetTalk) 25.0)) 1e+02)
              (Variables|Default|SetTalk 1e+02)
              (else
                (Variables|Default|SetTalk (Math|Random|RandomFloatinRange (- (Variables|Default|GetTalk) 25.0) (+ (Variables|Default|GetTalk) 25.0)))
                (goto _label Close)))))))
    (:then_1
      (Utilities|FlowControl|Delay 5.0)
      (goto _label Open))))

(fn ConstructionScript
  (bind _returnvalue (Utilities|GetDataTableRow "/Game/NUESTRO/BLUEPRINTS/QuestDT.QuestDT" "1")
    (:then
      (Variables|Default|SetActualQuest _returnvalue)
      (Rendering|Components|TextRender|SetText (Variables|Default|GetInstruccion) (.Narrativa (Utilities|Struct|BreakQuest _returnvalue))))))

(fn GetNextEnumIndex
  (params (Actual :type QuestRecompensa%20Enum :default "NewEnumerator0"))
  (bind _array (Utilities|Array|MakeArray "NewEnumerator0" "NewEnumerator1" "NewEnumerator2" "NewEnumerator3" "NewEnumerator4"))
  (bind _returnvalue (Utilities|Array|FindItem _array Actual))
  (bind _returnvalue_2 (+ _returnvalue 1))
  (if (<= _returnvalue_2 (Utilities|Array|Length _array))
    (return (Utilities|Array|Get(acopy) _array _returnvalue_2))
    (else
      (return (Utilities|Array|Get(acopy) _array _returnvalue)))))