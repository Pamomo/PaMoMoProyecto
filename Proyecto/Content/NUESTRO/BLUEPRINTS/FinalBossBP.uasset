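; Final boss that runs a dance-guessing battle once MainCharBP overlaps its Box, winning and pausing the game at five correct dances.
; Tick cycles through flags and Delays: it picks a hidden random dance, prompts "BAILA!!", then compares it with the player's BaileActual.
; A match adds to the score; a miss flags PlatFinalBattle platforms to fall, re-rolling the random index per platform, so the number dropped varies.
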(event OnComponentBeginOverlap(Box)
  (params (OverlappedComponent :type Primitive%20Component%20Object%20Reference) (OtherActor :type Actor%20Object%20Reference) (OtherComp :type Primitive%20Component%20Object%20Reference) (OtherBodyIndex :type Integer) (bFromSweep :type Boolean) (SweepResult :type Hit%20Result%20Structure%20%28by%20ref%29))
  (Utilities|Casting|CastToMainCharBP OtherActor)
  (Variables|Default|SetActivated true)
  (Variables|/Script/Engine.PrimitiveComponent|SetbGenerateOverlapEvents (Variables|Default|GetBox) false))

(event Custom|DesactivarPlataforma
  (bind _outactors (Actor|GetAllActorsOfClass "/Game/NUESTRO/BLUEPRINTS/PlatFinalBattle.PlatFinalBattle_C"))
  (for (_array_element _array_index) _outactors
    (if (== _array_index (Math|Random|RandomIntegerinRange 0 (Utilities|Array|Length _outactors)))
      (Variables|/Game/NUESTRO/BLUEPRINTS/PlatFinalBattle.PlatFinalBattle_C|SetHaveToFall _array_element true))))

(event EventTick
  (params (DeltaSeconds :type Float%20%28single-precision%29))
  (if (Variables|Default|GetActivated)
    (Variables|Default|SetPlayerWin (== (Variables|Default|GetBailesCorrectos) 5))
    (if (Variables|Default|GetPlayerWin)
      (Rendering|Components|TextRender|SetText (Variables|Default|GetTextRender) (Utilities|Text|MakeLiteralText "YOU WIN!!!"))
      (Game|SetGamePaused true)
      (else
        (Utilities|FlowControl|Sequence
          (:then_0
            (if (not (Variables|Default|GetBaileEscogido))
              (Variables|Default|SetDance (Math|Random|RandomIntegerinRange 1 5))
              (Rendering|Components|TextRender|SetText (Variables|Default|GetTextRender) (Utilities|Text|MakeLiteralText "BAILA!!"))
              (Variables|Default|SetBaileEscogido true)))
          (:then_1
            (if (Variables|Default|GetBaileEscogido)
              (if (not (Variables|Default|GetAlgoHecho))
                (Utilities|FlowControl|Delay 7.0)
                (bind _mismobaile (CallFunction|CheckBaile))
                (if _mismobaile
                  (Rendering|Components|TextRender|SetText (Variables|Default|GetTextRender) (Utilities|Text|MakeLiteralText "QUE SUERTE TIENES..."))
                  (bind _result (Math|Integer|IncrementInt (Variables|Default|GetBailesCorrectos))
                    (:%20%20
                      (Development|PrintString (Utilities|String|ToString(Integer) _result) true false "(R=0.000000,G=0.660000,B=1.000000,A=1.000000)" 1e+03)))
                  (else
                    (Rendering|Components|TextRender|SetText (Variables|Default|GetTextRender) (Utilities|Text|MakeLiteralText "FALLASTE!!"))
                    (CallFunction|DesactivarPlataforma)))
                (Variables|Default|SetAlgoHecho true))))
          (:then_2
            (if (Variables|Default|GetAlgoHecho)
              (Utilities|FlowControl|Delay 5.0)
              (Variables|Default|SetBaileEscogido false)
              (Variables|Default|SetAlgoHecho false))))))))

(fn ConstructionScript)

(fn CheckBaile
  (if (== (Variables|/Game/NUESTRO/BLUEPRINTS/MainCharBP.MainCharBP_C|GetBaileActual (.AsMain%20Char%20BP (Utilities|Casting|CastToMainCharBP (Game|GetPlayerCharacter 0)))) (Variables|Default|GetDance))
    (return true)
    (else
      (return false))))