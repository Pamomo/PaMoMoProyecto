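; Platform Blueprint for the final battle that drops away after the player steps on it, if flagged as the first base.
; When the main character overlaps its box, a first-base platform waits ten seconds and sets a fall flag.
; Tick watches that flag and calls Fall, which turns on physics simulation on the static mesh.
; Platforms without the first-base flag ignore the overlap, though the flag can still trigger a fall.
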(event OnComponentBeginOverlap(Box)
  (params (OverlappedComponent :type Primitive%20Component%20Object%20Reference) (OtherActor :type Actor%20Object%20Reference) (OtherComp :type Primitive%20Component%20Object%20Reference) (OtherBodyIndex :type Integer) (bFromSweep :type Boolean) (SweepResult :type Hit%20Result%20Structure%20%28by%20ref%29))
  (Utilities|Casting|CastToMainCharBP OtherActor)
  (if (Variables|Default|GetIsFirstBase)
    (Utilities|FlowControl|Delay 1e+01)
    (Variables|Default|SetHaveToFall true)))

(event Custom|Fall
  (Physics|SetSimulatePhysics (Variables|Default|GetStaticMesh) true))

(event EventTick
  (params (DeltaSeconds :type Float%20%28single-precision%29))
  (if (Variables|Default|GetHaveToFall)
    (CallFunction|Fall)))

(fn ConstructionScript)