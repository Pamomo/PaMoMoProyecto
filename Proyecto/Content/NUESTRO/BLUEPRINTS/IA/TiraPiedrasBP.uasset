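; Stone-throwing AI enemy Blueprint that turns toward the player and fires projectiles.
; RotarHaciaElPlayer rotates the capsule to the look-at rotation toward the MainCharBP player character.
; Disparar waits a fixed delay, then spawns a scaled-down Proyectil at PuntoDeSalida, passing the capsule's forward vector and an impulse for the launch.
; Neither event is triggered within this graph.
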(event Custom|Disparar
  (Utilities|FlowControl|Delay 3.0)
  (Game|SpawnActorfromClass "/Game/NUESTRO/BLUEPRINTS/IA/Proyectil.Proyectil_C" (Math|Transform|MakeTransform (Transformation|GetWorldLocation (Variables|Default|GetPuntoDeSalida)) (Transformation|GetWorldRotation (Variables|Character|GetMesh)) "0.300000,0.300000,0.300000") "Undefined" 0 (Math|Vector|GetForwardVector (Variables|Collision|GetCapsuleComponent)) 6e+03 0))

(event Custom|RotarHaciaElPlayer
  (Transformation|SetWorldRotation (Variables|Collision|GetCapsuleComponent) (Math|Rotator|FindLookatRotation (Transformation|GetActorLocation) (Transformation|GetActorLocation (.AsMain%20Char%20BP (Utilities|Casting|CastToMainCharBP (Game|GetPlayerCharacter 0))))) false false))

(fn ConstructionScript)