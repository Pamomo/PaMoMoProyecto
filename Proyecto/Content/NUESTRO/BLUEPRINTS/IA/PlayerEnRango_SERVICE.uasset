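; Behavior tree service that flags whether the player is within an AI's detection range.
; On each tick it measures the distance between the AI controller's pawn and the player's MainCharBP.
; It writes whether that distance is at most RangoDeDeteccion into the TargetDentroDelRango blackboard bool.
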(event EventTick
  (params (OwnerActor :type Actor%20Object%20Reference) (DeltaSeconds :type Float%20%28single-precision%29))
  (Class|BTFunctionLibrary|SetBlackboardValueasBool (Variables|Default|GetTargetDentroDelRango) (<= (Math|Vector|VectorLength (- (Transformation|GetActorLocation (Pawn|GetControlledPawn (.AsAIController (Utilities|Casting|CastToAIController OwnerActor)))) (Transformation|GetActorLocation (.AsMain%20Char%20BP (Utilities|Casting|CastToMainCharBP (Game|Player|GetPlayerPawn 0)))))) (Variables|Default|GetRangoDeDeteccion))))