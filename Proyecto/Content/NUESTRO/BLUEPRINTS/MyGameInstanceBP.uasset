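; Game instance that saves and loads player and progress state through MySaveGame in the "ElSave" slot.
; SaveGame stores transform, inventory, unlocked dances, progress flags, chicken count and game mode Life/Stamina, written to each other's fields.
; LoafGame restores these but resets Guitarra and Baguete to false, then changes game mode state.
; Loading destroys as many Pollo actors as were counted and rebuilds inventory by spawning ItemBP actors at the saved player transform.
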(event Custom|SaveGame
  (bind _returnvalue (Game|GetGameMode))
  (bind _returnvalue_2 (Game|GetGameInstance))
  (bind _returnvalue_3 (Game|GetPlayerCharacter 0))
  (bind _asmain_char_bp (Utilities|Casting|CastToMainCharBP _returnvalue_3))
  (bind _asmy_game_mode_bp (Utilities|Casting|CastToMyGameModeBP _returnvalue))
  (bind _asmy_game_instance_bp (Utilities|Casting|CastToMyGameInstanceBP _returnvalue_2))
  ;[1 1 1] Save Game
  (bind _returnvalue_4 (SaveGame|CreateSaveGameObject "/Game/NUESTRO/BLUEPRINTS/MySaveGame.MySaveGame_C"))
  (Variables|/Game/NUESTRO/BLUEPRINTS/MySaveGame.MySaveGame_C|SetPlayer%20Transform _returnvalue_4 (Transformation|GetActorTransform _asmain_char_bp))
  (for (_array_element _array_index) (Variables|/Game/NUESTRO/BLUEPRINTS/MainCharBP.MainCharBP_C|GetInventory _asmain_char_bp)
    (Utilities|Array|Insert (Variables|/Game/NUESTRO/BLUEPRINTS/MySaveGame.MySaveGame_C|GetPlayer%20Inventory _returnvalue_4) _array_element _array_index))
  (for (_array_element_2 _array_index_2) (Variables|/Game/NUESTRO/BLUEPRINTS/MainCharBP.MainCharBP_C|GetBailes%20Desbloqueados _asmain_char_bp)
    (Utilities|Array|SetArrayElem (Variables|/Game/NUESTRO/BLUEPRINTS/MySaveGame.MySaveGame_C|GetPlayer%20BailesDesbloqueados _returnvalue_4) _array_index_2 _array_element_2))
  (Variables|/Game/NUESTRO/BLUEPRINTS/MySaveGame.MySaveGame_C|SetGM%20Stamina _returnvalue_4 (Variables|/Game/NUESTRO/BLUEPRINTS/MyGameModeBP.MyGameModeBP_C|GetLife _asmy_game_mode_bp))
  (Variables|/Game/NUESTRO/BLUEPRINTS/MySaveGame.MySaveGame_C|SetGM%20Life _returnvalue_4 (Variables|/Game/NUESTRO/BLUEPRINTS/MyGameModeBP.MyGameModeBP_C|GetStamina _asmy_game_mode_bp))
  (Variables|/Game/NUESTRO/BLUEPRINTS/MySaveGame.MySaveGame_C|SetGI%20TodosLosPollos _returnvalue_4 (Variables|MyGameInstanceBP_C|GetTodosLosPollos _asmy_game_instance_bp))
  (Variables|/Game/NUESTRO/BLUEPRINTS/MySaveGame.MySaveGame_C|SetGI%20Pollos _returnvalue_4 (Variables|MyGameInstanceBP_C|GetPollos _asmy_game_instance_bp))
  (Variables|/Game/NUESTRO/BLUEPRINTS/MySaveGame.MySaveGame_C|SetGI%20PoderPerlas _returnvalue_4 (Variables|MyGameInstanceBP_C|GetPoderDeLasPerlas _asmy_game_instance_bp))
  (Variables|/Game/NUESTRO/BLUEPRINTS/MySaveGame.MySaveGame_C|SetGI%20Fisio _returnvalue_4 (Variables|MyGameInstanceBP_C|GetFisioCurado _asmy_game_instance_bp))
  (Variables|/Game/NUESTRO/BLUEPRINTS/MySaveGame.MySaveGame_C|SetGI%20Guitarra _returnvalue_4 (Variables|Default|GetGuitarra))
  (Variables|/Game/NUESTRO/BLUEPRINTS/MySaveGame.MySaveGame_C|SetGI%20Baguette _returnvalue_4 (Variables|Default|GetBaguete))
  (SaveGame|SaveGametoSlot _returnvalue_4 "ElSave"))

(event Custom|LoafGame
  (bind _returnvalue (Game|GetPlayerCharacter 0))
  (bind _returnvalue_2 (Game|GetGameMode))
  (bind _asmy_game_mode_bp (Utilities|Casting|CastToMyGameModeBP _returnvalue_2))
  (bind _asmain_char_bp (Utilities|Casting|CastToMainCharBP _returnvalue))
  (bind _returnvalue_3 (SaveGame|LoadGamefromSlot "ElSave"))
  (bind _asmy_save_game (Utilities|Casting|CastToMySaveGame _returnvalue_3))
  (Variables|/Game/NUESTRO/BLUEPRINTS/MyGameModeBP.MyGameModeBP_C|SetLife _asmy_game_mode_bp (Variables|/Game/NUESTRO/BLUEPRINTS/MySaveGame.MySaveGame_C|GetGM%20Life _asmy_save_game))
  (Variables|/Game/NUESTRO/BLUEPRINTS/MyGameModeBP.MyGameModeBP_C|SetStamina _asmy_game_mode_bp (Variables|/Game/NUESTRO/BLUEPRINTS/MySaveGame.MySaveGame_C|GetGM%20Stamina _asmy_save_game))
  (Variables|Default|SetGuitarra false)
  (Variables|Default|SetBaguete false)
  (Variables|Default|SetFisioCurado (Variables|/Game/NUESTRO/BLUEPRINTS/MySaveGame.MySaveGame_C|GetGI%20Fisio _asmy_save_game))
  (Variables|Default|SetPoderDeLasPerlas (Variables|/Game/NUESTRO/BLUEPRINTS/MySaveGame.MySaveGame_C|GetGI%20PoderPerlas _asmy_save_game))
  (Variables|Default|SetTodosLosPollos (Variables|/Game/NUESTRO/BLUEPRINTS/MySaveGame.MySaveGame_C|GetGI%20TodosLosPollos _asmy_save_game))
  (bind _output_get (Variables|Default|SetPollos (Variables|/Game/NUESTRO/BLUEPRINTS/MySaveGame.MySaveGame_C|GetGI%20Pollos _asmy_save_game)))
  (bind _outactors (Actor|GetAllActorsOfClass "/Game/NUESTRO/BLUEPRINTS/Pollo.Pollo_C"))
  (bind (_array_element _array_index) (Utilities|Array|ForEachLoopwithBreak _outactors :!label _label)
    (:LoopBody
      (if (< _array_index _output_get)
        (Actor|DestroyActor _array_element)
        (else
          (goto _label Break))))
    (:Completed
      (Transformation|SetActorTransform _asmain_char_bp (Variables|/Game/NUESTRO/BLUEPRINTS/MySaveGame.MySaveGame_C|GetPlayer%20Transform _asmy_save_game))
      (for (_array_element_2 _array_index_2) (Variables|/Game/NUESTRO/BLUEPRINTS/MySaveGame.MySaveGame_C|GetPlayer%20BailesDesbloqueados _asmy_save_game)
        (Utilities|Array|SetArrayElem (Variables|/Game/NUESTRO/BLUEPRINTS/MainCharBP.MainCharBP_C|GetBailes%20Desbloqueados _asmain_char_bp) _array_index_2 _array_element_2))
      (Utilities|Array|Clear (Variables|/Game/NUESTRO/BLUEPRINTS/MainCharBP.MainCharBP_C|GetInventory _asmain_char_bp))
      (for _array_element_3 (Variables|/Game/NUESTRO/BLUEPRINTS/MySaveGame.MySaveGame_C|GetPlayer%20Inventory _asmy_save_game)
        (if (Utilities|Name|NotEqual(Name) (.Item_Name (Utilities|Struct|BreakArma _array_element_3)) "None")
          (Game|SpawnActorfromClass "/Game/NUESTRO/INVENTORY/ItemBP.ItemBP_C" (Variables|/Game/NUESTRO/BLUEPRINTS/MySaveGame.MySaveGame_C|GetPlayer%20Transform _asmy_save_game) "Undefined" 0 (.NameDeLaRow (Utilities|Struct|BreakArma _array_element_3)) 0)))
      (Default|ChangeMode _asmy_game_mode_bp "NewEnumerator1"))))