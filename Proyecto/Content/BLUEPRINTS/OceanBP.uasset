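; OceanBP is an ocean actor that lays out a tiled grid of mesh instances.
; Its construction script runs nested loops over Width and Heigth, adding one Hierarchical Instanced Static Mesh instance per cell at a fixed spacing in local X and Y.
; The event graph holds only disabled stub events, so the Blueprint adds no runtime logic.
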(event EventBeginPlay)

(event Collision|EventActorBeginOverlap
  (params (OtherActor :type Actor%20Object%20Reference)))

(event EventTick
  (params (DeltaSeconds :type Float%20%28single-precision%29)))

(fn ConstructionScript
  (for _index (range 1 (Variables|Default|GetWidth))
    (for _index_2 (range 1 (Variables|Default|GetHeigth))
      (Components|InstancedStaticMesh|AddInstance (Variables|Default|GetHierarchicalInstancedStaticMesh) (Math|Transform|MakeTransform (Math|Vector|MakeVector (Math|Conversions|ToFloat(Integer) (* _index 2500)) (Math|Conversions|ToFloat(Integer) (* _index_2 2500)) 0.0))))))